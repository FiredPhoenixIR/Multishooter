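; BP_ApplyEffectZone is a trigger volume that grants a configurable action or effect to player characters entering it.
; On Box overlap it filters for SCharacter, then on authority only adds EffectClassToApply through the actor's SActionComponent with the zone as Instigator.
; The construction script sets the Text3D label from OverheadText.
; An unconnected chain in the event graph would briefly disable player input, but never runs.
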(event OnComponentBeginOverlap(Box)
  (params (OverlappedComponent :type Primitive%20Component%20Object%20Reference) (OtherActor :type Actor%20Object%20Reference) (OtherComp :type Primitive%20Component%20Object%20Reference) (OtherBodyIndex :type Integer) (bFromSweep :type Boolean) (SweepResult :type Hit%20Result%20Structure%20%28by%20ref%29))
  (bind _returnvalue (Actor|GetComponentbyClass OtherActor "/Script/ActionRoguelike.SActionComponent"))
  (Utilities|Casting|CastToSCharacter OtherActor) ; Basic check to filter only he player and skip bots.\n(Ideally use a gameplaytag or similar)
  (Networking|SwitchHasAuthority ; Only server/host is allowed to add actions
    (:Authority
      (Utilities|IsValid _returnvalue :!pinned true ; Ignore other overlaps like projectiles flying through\nthat dont have ActionComponent
        (:Is%20Valid
          (Class|SActionComponent|AddAction _returnvalue self (Variables|Default|GetEffectClassToApply)))))))

(fn ConstructionScript
  (Variables|/Script/Text3D.Text3DComponent|SetText (Variables|Default|GetText3D) (Variables|Default|GetOverheadText)))